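; BP_ItemBase is a base item actor Blueprint that exposes an item's tag, type and effect data through simple getters.
; GetItemData returns a damage radius with light-damage and stun effects.
; InitLeadPose, commented as fitting the item to a mesh's skeleton, only forwards the lead mesh to the parent implementation.
; The Blueprint's own SKItem leader-pose and location-reset nodes are disconnected and never run.
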(event EventBeginPlay)

(event Collision|EventActorBeginOverlap
  (params (OtherActor :type Actor%20Object%20Reference)))

(event EventTick
  (params (DeltaSeconds :type Float%20%28single-precision%29)))

(event EventInitLeadPose
  (params (LeadMesh :type Skeletal%20Mesh%20Component%20Object%20Reference))
  (|CallParentFunction LeadMesh))

(fn ConstructionScript)

(fn GetItemTag
  (return (Variables|Default|GetTag)))

(fn GetItemType
  (return (Variables|Default|GetItemType)))

(fn GetItemData
  (return (Variables|Default|GetDamageRadius) 0 (Variables|Default|GetGE_Damage_lite) (Variables|Default|GetGE_Stun)))