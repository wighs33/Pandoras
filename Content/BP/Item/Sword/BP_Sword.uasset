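; BP_Sword is a melee weapon item that applies GAS damage and stun through hitbox overlaps.
; BeginPlay loads damage and effect classes from the item DataTable row named after its class.
; Overlaps box-trace for the hit actor, send hit-react events, then apply SetByCaller damage, doubled when charged, unless the target is evading; evading-and-blocking targets get block FX.
; RepNotify flags mirror trail and blood effects; charging briefly tints the material red.
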(event EventBeginPlay
  (|CallParentFunction)
  ;[0.15 0.15 0.15 0.5] 히트박스 감지 끄기
  (Class|ItemInterface|ToggleHitBox false)
  ;[0.15 0.15 0.15 0.5] 아이템 데이터 테이블에서 '이 클래스 이름'을 키로 가지는 데이터 얻기
  (bind _returnvalue (Utilities|GetDataTableRow (Variables|Default|GetDT_Item) (Utilities|String|StringToName (Utilities|String|Replace (Utilities|GetClassDisplayName (Utilities|GetClass self)) "_C")))
    (:then
      ;[0.15 0.15 0.15 0.5] 데미지, GE를 뽑아와서 저장
      (if (.ReturnValue (Utilities|Map|Find (.WeaponStats (Utilities|Struct|BreakWeaponProperties (.WeaponProperties (Utilities|Struct|BreakItemData _returnvalue)))) "Attack"))
        (Variables|Default|SetDamageAmount (* (Math|Conversions|ToFloat(Integer) (.Value (Utilities|Map|Find (.WeaponStats (Utilities|Struct|BreakWeaponProperties (.WeaponProperties (Utilities|Struct|BreakItemData _returnvalue)))) "Attack"))) -1.0))
        (Variables|Default|SetGE_Damage_lite (Utilities|ResolveSoftReference (.GEDamage (Utilities|Struct|BreakWeaponProperties (.WeaponProperties (Utilities|Struct|BreakItemData _returnvalue))))))
        (Variables|Default|SetGE_Stun (Utilities|ResolveSoftReference (.GEStun (Utilities|Struct|BreakWeaponProperties (.WeaponProperties (Utilities|Struct|BreakItemData _returnvalue))))))))))

(event Collision|EventActorBeginOverlap
  (params (OtherActor :type Actor%20Object%20Reference)))

(event EventOnHitBoxBeginOverlap
  (params (OverlappedComp :type Primitive%20Component%20Object%20Reference) (OtherActor :type Actor%20Object%20Reference) (OtherComp :type Primitive%20Component%20Object%20Reference) (OtherBodyIndex :type Integer) (bFromSweep :type Boolean) (SweepResult :type Hit%20Result%20Structure%20%28by%20ref%29))
  (bind _hitactor (Variables|Default|GetHitActor))
  (bind _hitactor_2 (Variables|Default|GetHitActor))
  (bind _damageamount (Variables|Default|GetDamageAmount))
  (bind _returnvalue (Ability|GetAbilitySystemComponent _hitactor_2))
  (bind _returnvalue_2 (Ability|GetAbilitySystemComponent _hitactor))
  ;[0.15 0.15 0.15 0.5] 감지된 액터가 지금여기의 검이 아닌 지 체크
  (if (!= OtherActor (Actor|GetAttachParentActor))
    (Development|PrintString "Damaging")
    ;[0.15 0.15 0.15 0.5] 액터 감지
    (|DetermineContactPointandActor OtherComp)
    ;[0.15 0.15 0.15 0.5] 피격된 액터의 피격 반응
    (Class|CharacterGameAbilityInterface|SendGameplayEventReplicated(Message) (Game|GetPlayerCharacter 0) (Variables|Default|GetHitActor) (select (Variables|Default|GetWeaponCharged) "(TagName=\"Character.Event.HitReact.Charged\")" "(TagName=\"Character.Event.HitReact.Lite\")") (Utilities|Struct|MakeGameplayEventData (Actor|GetAttachParentActor)))
    ;[0.15 0.15 0.15 0.5] 피격된 액터가 회피 중이거나 블로킹 중인지 체크
    (if (GameplayTags|HasAnyMatchingGameplayTags _returnvalue_2 (GameplayTags|MakeLiteralGameplayTagContainer "(GameplayTags=((TagName=\"Character.State.Evading\"),(TagName=\"Character.State.Blocking\")))"))
      ;[0.15 0.15 0.15 0.5] 피격된 액터가 블로킹 중인지 체크
      (if (GameplayTags|HasAnyMatchingGameplayTags _returnvalue_2 (GameplayTags|MakeLiteralGameplayTagContainer "(GameplayTags=((TagName=\"Character.State.Blocking\")))"))
        ;[0.15 0.15 0.15 0.5] 블락 이펙트 재생
        (Niagara|SpawnSystematLocation "/Game/VFX/Particles/Blockable/NS_Blocked.NS_Blocked" (Variables|Default|GetContactLocation))
        ;[0.15 0.15 0.15 0.5] 사운드 재생
        (Audio|PlaySoundatLocation (Variables|Default|GetBlockedSound) (Transformation|GetActorLocation) "0, 0, 0" 1.0 1.0 0.0 0 0 0 0))
      (else
        ;[0.15 0.15 0.15 0.5] 데이터테이블에서 얻은 GE에서 데미지값을 설정 후에 사용
        (bind _returnvalue_3 (Ability|GameplayEffect|AssignTagSetbyCallerMagnitude (GameplayEffects|MakeOutgoingSpec :self _returnvalue_2 :GameplayEffectClass (Variables|Default|GetGE_Damage_lite)) (Variables|Default|GetDamageTag) (select (Variables|Default|GetWeaponCharged) (* _damageamount 2.0) _damageamount)))
        (GameplayEffects|ApplyGameplayEffectSpecToTarget _returnvalue_2 _returnvalue_3 _returnvalue_2)
        ;[0.15 0.15 0.15 0.5] 스턴
        (if (not (GameplayTags|HasAnyMatchingGameplayTags _returnvalue (GameplayTags|MakeLiteralGameplayTagContainer "(GameplayTags=((TagName=\"Character.State.Evading\")))")))
          (GameplayEffects|ApplyGameplayEffectToTarget :self _returnvalue :GameplayEffectClass (Variables|Default|GetGE_Stun) :Target _returnvalue))))))

(event EventOnBlockBoxBeginOverlap
  (params (OverlappedComp :type Primitive%20Component%20Object%20Reference) (OtherActor :type Actor%20Object%20Reference) (OtherComp :type Primitive%20Component%20Object%20Reference) (OtherBodyIndex :type Integer) (bFromSweep :type Boolean) (SweepResult :type Hit%20Result%20Structure%20%28by%20ref%29)))

(event EventToggleBlockBox
  (params (Enable :type Boolean))
  (|CallParentFunction Enable))

(event EventTick
  (params (DeltaSeconds :type Float%20%28single-precision%29)))

(event EventToggleSwordTrail
  (params (Enable :type Boolean))
  (bind _trailfx (Variables|Default|GetTrailFx))
  ;[0.15 0.15 0.15 0.5] 플래그에 따라 활성화여부 결정 (리플리케이션)
  (bind _output_get (Variables|Default|SetTrailEnabled Enable))
  (if _output_get
    (Components|Activation|Activate _trailfx false)
    ;[0.15 0.15 0.15 0.5] 검 휘두르는 소리 재생
    (Audio|PlaySoundatLocation (Variables|Default|GetSwingSound) (Transformation|GetActorLocation) "0, 0, 0" 1.0 1.0 0.0 0 0 0 0)
    (else
      (Components|Activation|Deactivate _trailfx))))

(event EventTriggerBlood
  ;[0.15 0.15 0.15 0.5] 플래그 ON
  (Variables|Default|SetBloodTriggered true)
  ;[0.15 0.15 0.15 0.5] 활성화
  (Components|Activation|Activate (Variables|Default|GetBloodFx) false)
  ;[0.15 0.15 0.15 0.5] 피격 사운드 재생
  (Audio|PlaySoundatLocation (Variables|Default|GetHitSound) (Transformation|GetActorLocation) "0, 0, 0" 1.0 1.0 0.0 0 0 0 0)
  ;[0.15 0.15 0.15 0.5] 랜덤 시간 후 비활성화
  (Utilities|FlowControl|Delay (Math|Random|RandomFloatinRange 0.05 0.15))
  (Components|Activation|Deactivate (Variables|Default|GetBloodFx))
  ;[0.15 0.15 0.15 0.5] 플래그 OFF
  (Variables|Default|SetBloodTriggered false))

(event EventDrop
  (|CallParentFunction))

(event EventChargeWeapon
  ;[0.15 0.15 0.15 0.5] 머티리얼 내 파라미터를 빨간색으로 변경
  (Rendering|Material|SetVectorParameterValueonMaterials (Variables|Default|GetSK_Item) "ChargedColor" (Math|Conversions|ToVector(LinearColor) "(R=1.000000,G=0.000000,B=0.000000,A=1.000000)"))
  ;[0.15 0.15 0.15 0.5] 플래그 ON
  (Variables|Default|SetWeaponCharged true)
  ;[0.15 0.15 0.15 0.5] 0.7초 후 머티리얼 내 파라미터를 검정색으로 복구
  (Utilities|FlowControl|RetriggerableDelay 0.7)
  (Rendering|Material|SetVectorParameterValueonMaterials (Variables|Default|GetSK_Item) "ChargedColor" (Math|Conversions|ToVector(LinearColor) "(R=0.000000,G=0.000000,B=0.000000,A=1.000000)"))
  ;[0.15 0.15 0.15 0.5] 플래그 OFF
  (Variables|Default|SetWeaponCharged false))

(event EventToggleHitBox
  (params (Enable :type Boolean))
  (|CallParentFunction Enable))

(event EventOnRepBloodTriggered
  (bind _bloodfx (Variables|Default|GetBloodFx))
  ;[0.15 0.15 0.15 0.5] OnRep
  (if (Variables|Default|GetBloodTriggered)
    (Components|Activation|Activate _bloodfx false)
    (else
      (Components|Activation|Deactivate _bloodfx))))

(event EventOnRepTrailEnabled
  (bind _trailfx (Variables|Default|GetTrailFx))
  ;[0.15 0.15 0.15 0.5] OnRep
  (if (Variables|Default|GetTrailEnabled)
    (Components|Activation|Activate _trailfx false)
    (else
      (Components|Activation|Deactivate _trailfx))))

(fn ConstructionScript)

(fn GetItemType
  (return (Variables|Default|GetItemType)))

(fn GetItemData
  (return 0.0 0 0 0))