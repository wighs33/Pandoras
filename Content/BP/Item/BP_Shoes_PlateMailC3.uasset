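; BP_Shoes_PlateMailC3 is a plate mail footwear item whose SKItem and Pads meshes follow the pose of a supplied lead mesh.
; Its InitLeadPose event zeroes the relative location of both components and sets the passed LeadMesh as their leader pose component.
; BeginPlay, overlap and Tick are disabled stubs, and the construction script only calls its parent.
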(event EventBeginPlay
  (|CallParentFunction) ; This node is disabled and will not be called.\nDrag off pins to build functionality.
)

(event Collision|EventActorBeginOverlap
  (params (OtherActor :type Actor%20Object%20Reference))
  (|CallParentFunction OtherActor) ; This node is disabled and will not be called.\nDrag off pins to build functionality.
)

(event EventTick
  (params (DeltaSeconds :type Float%20%28single-precision%29))
  (|CallParentFunction DeltaSeconds) ; This node is disabled and will not be called.\nDrag off pins to build functionality.
)

(event EventInitLeadPose
  (params (LeadMesh :type Skeletal%20Mesh%20Component%20Object%20Reference))
  (bind _sk_item (Variables|Default|GetSK_Item))
  (Transformation|SetRelativeLocation _sk_item "0, 0, 0" false false)
  (Components|SkinnedMesh|SetLeaderPoseComponent _sk_item LeadMesh false false))

(fn ConstructionScript
  (|CallParentFunction))