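; BP_PandorasPlayerController is a player controller that handles input focus and toggles between the in-game HUD and skill menu.
; It starts in game-only input, and a FlipFlop on K messages the HUD to switch screens while toggling pawn input and input mode.
; Opening the menu shows the mouse cursor, but closing it never hides it again.
; GetKeyName joins the display names of keys mapped to an Enhanced Input action into one string.
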(event EventBeginPlay
  (|CallParentFunction)
  (Input|SetInputModeGameOnly self false) ; 게임 입력 모드로 설정 (시작할 때 뷰포트 포커싱)
)

(event EventTick
  (params (DeltaSeconds :type Float%20%28single-precision%29)))

(event Input|KeyboardEvents|K
  (params (Key :type Key%20Structure :default "None"))
  (bind _returnvalue (HUD|GetHUD))
  (bind _returnvalue_2 (Pawn|GetControlledPawn))
  (bind _self self)
  (bind _self_2 self)
  (:Pressed
    ;[0.15 0.15 0.15 0.5] 스킬메뉴와 HUD 전환
    (Utilities|FlowControl|FlipFlop
      (:A
        (Class|HudInterface|SwitchtoSkillMenu(Message) _returnvalue)
        ;[0.15 0.15 0.15 0.5] 폰의 입력 활성화 전환
        (Input|DisableInput _returnvalue_2 _self)
        ;[0.15 0.15 0.15 0.5] 입력 모드 전환
        (Input|SetInputModeGameandUI _self_2 0 "DoNotLock" false false)
        ;[0.15 0.15 0.15 0.5] 마우스 커서 등장
        (Variables|Default|SetbShowMouseCursor true))
      (:B
        (Class|HudInterface|SwitchtoinGameHud(Message) _returnvalue)
        (Input|EnableInput _returnvalue_2 _self)
        (Input|SetInputModeGameOnly _self_2 false)))))

(fn ConstructionScript)

(fn GetKeyName
  (params (Input :type Input%20Action%20Object%20Reference))
  ;[0.15 0.15 0.15 0.5] 지정된 액션과 매핑된 키들 각각
  (for _array_element (Class|EnhancedInputSubsystemInterface|QueryKeysMappedtoAction (PlayerController|LocalPlayerSubsystems|GetEnhancedInputLocalPlayerSubsystem) Input)
    ;[0.15 0.15 0.15 0.5] 매핑된 키들을 하나의 문자열로 이어붙임
    (LocalVariables|SetKeyNames (Utilities|String|Append (LocalVariables|GetKeyNames) (Utilities|String|ToString(Text) (Class|KismetInputLibrary|KeyGetDisplayName _array_element false)))))
  ;[0.15 0.15 0.15 0.5] 완성된 문자열 반환
  (return (LocalVariables|GetKeyNames)))