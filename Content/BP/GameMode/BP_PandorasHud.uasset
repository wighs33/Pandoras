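; Player HUD that owns the main UI widget and switches between the in-game HUD, inventory, item list and skill tree screens.
; BeginPlay creates the main widget and caches its child screens for the switch events.
; Inventory screens refocus an InventoryRoom camera by item type, with item lists filled from PlayerState.
; It also toggles UI input mode, forwards health, stamina and notifications, and shows timed tips and level display via retriggerable delays.
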(event EventBeginPlay
  ;[0.15 0.15 0.15 0.5] 오너의 메인 UI 위젯(모든 화면 포함) 생성 후 저장
  (bind _returnvalue (UserInterface|CreateWidget "/Game/BP/UI/WDG_MainUI.WDG_MainUI_C" (Game|GetPlayerController 0)))
  (bind _output_get (Variables|Default|SetMainUIWidget _returnvalue))
  ;[0.15 0.15 0.15 0.5] 화면에 띄우기
  (UserInterface|Viewport|AddtoViewport _output_get 0)
  ;[0.15 0.15 0.15 0.5] 메인 UI 위젯에서 위젯들 가지고 와서 저장
  (|InitializeWidgetVariables))

(event Collision|EventActorBeginOverlap
  (params (OtherActor :type Actor%20Object%20Reference)))

(event EventUpdateStamina
  (params (Stamina :type Float%20%28single-precision%29))
  ;[0.15 0.15 0.15 0.5] HUD의 스태미나 갱신
  (bind _wdg_ingamehud (Variables|Default|GetWDG_InGameHud)
    (:then
      (Class|InGameHudWidget|UpdateStamina _wdg_ingamehud Stamina))
    (:else)))

(event EventShowTip
  (params (TipText :type String) (DisplayTime :type Float%20%28single-precision%29))
  ;[0.15 0.15 0.15 0.5] HUD가 유효하면 팁 보여주기
  (bind _wdg_ingamehud (Variables|Default|GetWDG_InGameHud)
    (:then
      (Default|ShowTip _wdg_ingamehud (Utilities|Text|ToText(String) TipText))
      ;[0.15 0.15 0.15 0.5] 설정한 시간만큼 딜레이
      (Utilities|FlowControl|RetriggerableDelay DisplayTime)
      ;[0.15 0.15 0.15 0.5] 팁 숨기기
      (Default|HideTip (Variables|Default|GetWDG_InGameHud)))
    (:else)))

(event EventSwitchtoSkillMenu
  ;[0.15 0.15 0.15 0.5] 유효성 체크 후 전환
  (bind _wdg_skilltree (Variables|Default|GetWDG_SkillTree)
    (:then
      (Class|MainUIWidget|SwitchWidget (Variables|Default|GetMainUIWidget) _wdg_skilltree)
      ;[0.15 0.15 0.15 0.5] 스킬 트리 리프레시
      (Class|SkillTreeWidget|RefreshSkillTree _wdg_skilltree))
    (:else)))

(event EventTick
  (params (DeltaSeconds :type Float%20%28single-precision%29)))

(event EventSwitchtoItemListUI
  (params (ItemType :type EItem%20Enum :default "UnArmed"))
  ;[0.15 0.15 0.15 0.5] 아이템 리스트 위젯 저장 후 이 위젯으로 화면 전환
  (Variables|Default|GetWDG_ItemList
    (:then
      (Class|MainUIWidget|SwitchWidget (Variables|Default|GetMainUIWidget) (Variables|Default|GetWDG_ItemList))
      ;[0.15 0.15 0.15 0.5] 타입에 맞는 아이템 클래스 리스트 가져오기
      (bind _returnvalue (Class|PlayerStateInterface|GetItemAbilityClassesbyType(Message) (Variables|/Script/Engine.Pawn|GetPlayerState (Game|GetPlayerCharacter 0)) ItemType))
      ;[0.15 0.15 0.15 0.5] 아이템 목록UI에 아이템 채우기
      (Class|ItemListWidget|InitItems (Variables|Default|GetWDG_ItemList) _returnvalue)
      ;[0.15 0.15 0.15 0.5] 아이템 타입 별로 카메라를 알맞은 위치에 포커싱
      (Class|InventoryRoom|ChangeFocusPoint (Variables|Default|GetInventoryRoom) (Utilities|Select :Index ItemType :UnArmed "Main" :Sword "Weapon" :GreatSword "Weapon" :Bow "Weapon" :Helmet "Head" :Armor "Main" :Glove "Hands" :Shoes "Feet")))
    (:else)))

(event EventShowRightNotification
  (params (NotificationData :type Notification%20Structure))
  ;[0.15 0.15 0.15 0.5] HUD의 알림 추가
  (Default|EnqueueNotification (Variables|/Game/BP/UI/WDG_InGameHud.WDG_InGameHud_C|GetWDG_RightNotification (Variables|Default|GetWDG_InGameHud)) NotificationData))

(event EventSwitchtoinGameHud
  ;[0.15 0.15 0.15 0.5] 인게임 HUD로 전환
  (Class|MainUIWidget|SwitchWidget (Variables|Default|GetMainUIWidget) (Variables|Default|GetWDG_InGameHud)))

(event EventSwitchtoInventoryUI
  (params (inventory_room :type Inventory%20Room%20Object%20Reference))
  ;[0.15 0.15 0.15 0.5] 인벤토리 룸 액터 저장
  (Variables|Default|GetInventoryRoom
    (:then
      _)
    (:else
      (Utilities|IsValid inventory_room
        (:Is%20Valid
          (Variables|Default|SetInventoryRoom inventory_room)))))
  ;[0.15 0.15 0.15 0.5] 인벤토리 메인 UI 화면으로 전환
  (bind _wdg_inventorymain (Variables|Default|GetWDG_InventoryMain)
    (:then
      (Class|MainUIWidget|SwitchWidget (Variables|Default|GetMainUIWidget) _wdg_inventorymain)
      ;[0.15 0.15 0.15 0.5] 레벨UI의 수치 갱신
      (Default|RefreshLevel (Variables|/Script/Pandoras.InventoryMainWidget|GetWDG_Level _wdg_inventorymain))
      ;[0.15 0.15 0.15 0.5] 카메라를 메인 위치에 포커싱
      (Class|InventoryRoom|ChangeFocusPoint (Variables|Default|GetInventoryRoom) "Main"))
    (:else)))

(event EventShowCharacterLevel
  (params (ShowDuration :type Float%20%28single-precision%29))
  ;[0.15 0.15 0.15 0.5] 레벨UI가 없으면 생성해서 뷰포트에 표시
  (Variables|Default|GetWDG_CharacterLevel
    (:then
      _)
    (:else
      (bind _returnvalue (UserInterface|CreateWidget "/Game/BP/UI/WDG_Level.WDG_Level_C"))
      (Variables|Default|SetWDG_CharacterLevel _returnvalue)))
  (UserInterface|Viewport|AddtoViewport (Variables|Default|GetWDG_CharacterLevel) 0)
  ;[0.15 0.15 0.15 0.5] 레벨UI의 수치 갱신
  (Default|RefreshLevel (Variables|Default|GetWDG_CharacterLevel))
  (Utilities|FlowControl|RetriggerableDelay ShowDuration)
  ;[0.15 0.15 0.15 0.5] 레벨UI를 화면에서 제거
  (Widget|RemovefromParent (Variables|Default|GetWDG_CharacterLevel)))

(event EventToggleUIInput
  (params (bInput :type Boolean))
  (bind _returnvalue (Game|GetPlayerController 0))
  ;[0.15 0.15 0.15 0.5] UI입력 플래그 체크
  (if bInput
    ;[0.15 0.15 0.15 0.5] 컨트롤러를 게임 및 ui모드로 바꾸고 마우스 커서 ON
    (Input|SetInputModeGameandUI _returnvalue 0 "DoNotLock" true false)
    (Variables|/Script/Engine.PlayerController|SetbShowMouseCursor _returnvalue true)
    (else
      ;[0.15 0.15 0.15 0.5] 컨트롤러를 게임전용모드로 바꾸고 마우스 커서 OFF
      (Input|SetInputModeGameOnly _returnvalue false)
      (Variables|/Script/Engine.PlayerController|SetbShowMouseCursor _returnvalue false))))

(event EventUpdateHealth
  (params (Health :type Float%20%28single-precision%29))
  ;[0.15 0.15 0.15 0.5] HUD의 체력바 갱신
  (bind _wdg_ingamehud (Variables|Default|GetWDG_InGameHud)
    (:then
      (Class|InGameHudWidget|UpdateHealth _wdg_ingamehud Health))
    (:else)))

(fn ConstructionScript)

(fn CheckActiveWidgetIsHudorInventory
  (return (== (Class|WidgetSwitcher|GetActiveWidgetIndex (Variables|/Script/Pandoras.MainUIWidget|GetWidgetSwitcher (Variables|Default|GetMainUIWidget))) 0)))