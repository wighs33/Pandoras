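; Player state that keeps a player's item-equip Gameplay Ability classes, sorted by item type.
; AddItemClass reads the item class from the ability's class defaults, then adds the ability uniquely to the array matching that item's type.
; Swords and great swords share one array, while bows and each armor slot have their own.
; Getter functions return the array for a given type or all arrays appended into one list.
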(event EventBeginPlay)

(event EventTick
  (params (DeltaSeconds :type Float%20%28single-precision%29)))

(event EventAddItemClass
  (params (itemAbility :type GA%20Equip%20Class%20Reference))
  (bind _itemclass (Utilities|GetClassDefaults itemAbility))
  ;[0.15 0.15 0.15 0.5] GA에 매칭된 아이템 클래스의 유효성 체크
  (if (Utilities|IsValidClass _itemclass)
    ;[0.15 0.15 0.15 0.5] 타입 별로 매칭되는 배열에 저장
    (switch Utilities|FlowControl|Switch|SwitchonEItem (.ItemType (Utilities|GetClassDefaults _itemclass))
      (:Sword
        (Utilities|Array|AddUnique (Variables|Default|GetSwordAbilityClasses) itemAbility :!label _label))
      (:GreatSword
        (goto _label))
      (:Bow
        (Utilities|Array|AddUnique (Variables|Default|GetBowAbilityClasses) itemAbility))
      (:Helmet
        (Utilities|Array|AddUnique (Variables|Default|GetHelmetAbilityClasses) itemAbility))
      (:Armor
        (Utilities|Array|AddUnique (Variables|Default|GetArmorAbilityClasses) itemAbility))
      (:Glove
        (Utilities|Array|AddUnique (Variables|Default|GetGlovesAbilityClasses) itemAbility))
      (:Shoes
        (Utilities|Array|AddUnique (Variables|Default|GetShoesAbilityClasses) itemAbility)))))

(fn ConstructionScript)

(fn GetItemAbilityClassesbyType
  (params (ItemType :type EItem%20Enum :default "UnArmed"))
  (bind _swordabilityclasses (Variables|Default|GetSwordAbilityClasses))
  (return (Utilities|Select :Index ItemType :UnArmed 0 :Sword _swordabilityclasses :GreatSword _swordabilityclasses :Bow (Variables|Default|GetBowAbilityClasses) :Helmet (Variables|Default|GetHelmetAbilityClasses) :Armor (Variables|Default|GetArmorAbilityClasses) :Glove (Variables|Default|GetGlovesAbilityClasses) :Shoes (Variables|Default|GetShoesAbilityClasses))))

(fn GetAllItemAbilities
  (bind _allclasses (LocalVariables|GetAllClasses))
  ;[0.15 0.15 0.15 0.5] 모든 아이템들을 저장하는 통합 아이템 리스트 채우기
  (Utilities|Array|AppendArray _allclasses (Variables|Default|GetSwordAbilityClasses))
  (Utilities|Array|AppendArray _allclasses (Variables|Default|GetBowAbilityClasses))
  (Utilities|Array|AppendArray _allclasses (Variables|Default|GetHelmetAbilityClasses))
  (Utilities|Array|AppendArray _allclasses (Variables|Default|GetArmorAbilityClasses))
  (Utilities|Array|AppendArray _allclasses (Variables|Default|GetGlovesAbilityClasses))
  (Utilities|Array|AppendArray _allclasses (Variables|Default|GetShoesAbilityClasses))
  (return (LocalVariables|GetAllClasses)))