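; Last-seen marker actor that shows a frozen copy of the player's pose at the player's transform.
; ToggleSnapshot points ABP_Snapshot's source mesh at the player mesh, moves the actor there, then pauses animation after a brief delay to hold the pose.
; Retriggerable delays reveal the snapshot shortly afterwards if still requested, then hide it again.
; It starts hidden, and toggling off hides it immediately.
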(event EventBeginPlay
  ;[0.15 0.15 0.15 0.5] 스냅샷 보여주기 토글
  (Class|LastSeen|ToggleSnapshot false))

(event Collision|EventActorBeginOverlap
  (params (OtherActor :type Actor%20Object%20Reference)))

(event EventTick
  (params (DeltaSeconds :type Float%20%28single-precision%29)))

(event EventToggleSnapshot
  (params (NewShowOrHide :type Boolean))
  (bind _returnvalue (Game|GetPlayerCharacter 0))
  (bind _sk_snapshot (Variables|Default|GetSK_Snapshot))
  ;[0.15 0.15 0.15 0.5] 보여줄지 숨길지 체크
  (bind _output_get (Variables|Default|SetShowOrHide NewShowOrHide))
  (if _output_get
    ;[0.15 0.15 0.15 0.5] 애니메이션 정지하고 애님 블루프린트 가져오기
    (Variables|/Script/Engine.SkeletalMeshComponent|SetbPauseAnims _sk_snapshot false)
    (bind _asabp_snapshot (Utilities|Casting|CastToABP_Snapshot (Components|SkeletalMesh|GetAnimInstance _sk_snapshot)))
    ;[0.15 0.15 0.15 0.5] ABP의 Source Mesh Component 변수를 플레이어 캐릭터의 메시로 설정
    (Variables|/Script/Pandoras.SnapshotAnimInstance|SetSourceMeshComponent _asabp_snapshot (Variables|/Script/Engine.Character|GetMesh _returnvalue))
    ;[0.15 0.15 0.15 0.5] 플레이어의 캐릭터의 트랜스폼으로 맞추기
    (Transformation|SetActorTransform (Transformation|GetActorTransform _returnvalue))
    (Utilities|FlowControl|Delay 0.2)
    ;[0.15 0.15 0.15 0.5] 애니메이션 중지
    (Variables|/Script/Engine.SkeletalMeshComponent|SetbPauseAnims (Variables|Default|GetSK_Snapshot) true)
    (Utilities|FlowControl|RetriggerableDelay 2.0)
    ;[0.15 0.15 0.15 0.5] 보여주기로 지정되었을 때 인게임 내에 보여주기
    (if (Variables|Default|GetShowOrHide)
      (Rendering|SetActorHiddenInGame false)
      (Utilities|FlowControl|RetriggerableDelay 3.0)
      ;[0.15 0.15 0.15 0.5] 인게임에서 숨기기
      (Rendering|SetActorHiddenInGame true))
    (else
      ;[0.15 0.15 0.15 0.5] 숨기기
      (Rendering|SetActorHiddenInGame true))))

(fn ConstructionScript)