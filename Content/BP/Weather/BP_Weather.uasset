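; Weather actor that drives sky Rayleigh scattering, post-process exposure and volumetric cloud coverage for clear and rainy looks.
; Dark and Clear apply presets instantly, while SetAtmosphereTargetParameter enables Tick to interpolate at constant speed until exposure reaches its target.
; StartRain runs a self-repeating timed cycle that darkens the atmosphere, toggles the referenced Rain on and off, then clears.
; SetAtmosphereValues applies values to the referenced actors, lazily creating the cloud dynamic material.
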(event Custom|Dark
  (CallFunction|SetAtmosphereValues "(R=0.200000,G=0.200000,B=0.200000,A=1.000000)" -1.0 0.0))

(event Custom|Clear
  (CallFunction|SetAtmosphereValues "(R=0.175287,G=0.409607,B=1.000000,A=1.000000)" 1.0 -0.2))

(event Custom|SetAtmosphereTargetParameter
  (params (Target%20Cloud%20Density%20Offset :type Float%20%28single-precision%29) (Target%20Exposure%20Compensation :type Float%20%28single-precision%29) (Target%20Rayleigh%20Scattering :type Linear%20Color%20Structure))
  (Variables|AtmosphereValue|SetTarget%20Cloud%20Density%20Offset Target%20Cloud%20Density%20Offset)
  (Variables|AtmosphereValue|SetTarget%20Exposure%20Compensation Target%20Exposure%20Compensation)
  (Variables|AtmosphereValue|SetTarget%20Rayleigh%20Scattering Target%20Rayleigh%20Scattering)
  (Actor|Tick|SetActorTickEnabled true))

(event Custom|ToggleRain)

(event Custom|StartRain
  (Utilities|FlowControl|Delay 2.0)
  (CallFunction|SetAtmosphereTargetParameter 0.0 -1.0 "(R=0.200000,G=0.200000,B=0.200000,A=1.000000)")
  (Utilities|FlowControl|Delay 15.0)
  (bind _rain (Variables|Default|GetRain)
    (:then
      (Default|ToggleRain _rain true)
      (Utilities|FlowControl|Delay 6e+01)
      (Default|ToggleRain (Variables|Default|GetRain) false)
      (Utilities|FlowControl|Delay 5.0)
      (CallFunction|SetAtmosphereTargetParameter -0.2 1.0 "(R=0.174647,G=0.407240,B=1.000000,A=1.000000)")
      (CallFunction|StartRain))
    (:else)))

(event EventBeginPlay)

(event Collision|EventActorBeginOverlap
  (params (OtherActor :type Actor%20Object%20Reference)))

(event EventTick
  (params (DeltaSeconds :type Float%20%28single-precision%29))
  (bind _returnvalue (Math|Float|MakeLiteralFloat 0.05))
  (bind _exposure_compensation (Variables|AtmosphereValue|GetExposure%20Compensation))
  (bind _target_exposure_compensation (Variables|AtmosphereValue|GetTarget%20Exposure%20Compensation))
  (CallFunction|SetAtmosphereValues (CallFunction|ColorInterptoConstant (Variables|AtmosphereValue|GetRayleigh%20Scattering) (Variables|AtmosphereValue|GetTarget%20Rayleigh%20Scattering) _returnvalue) (Math|Interpolation|FInterptoConstant _exposure_compensation _target_exposure_compensation DeltaSeconds _returnvalue) (Math|Interpolation|FInterptoConstant (Variables|AtmosphereValue|GetCloud%20Density%20Offset) (Variables|AtmosphereValue|GetTarget%20Cloud%20Density%20Offset) DeltaSeconds _returnvalue))
  (Actor|Tick|SetActorTickEnabled (not (Math|Float|NearlyEqual(Float) _exposure_compensation _target_exposure_compensation 1e-06))))

(fn ConstructionScript)

(fn SetAtmosphereValues
  (params (Rayleigh%20Scattering :type Linear%20Color%20Structure) (Exposure%20Compensation :type Float%20%28single-precision%29) (CloudDensityOffset :type Float%20%28single-precision%29))
  (Variables|AtmosphereValue|SetCloud%20Density%20Offset CloudDensityOffset)
  (Variables|AtmosphereValue|SetExposure%20Compensation Exposure%20Compensation)
  (Variables|AtmosphereValue|SetRayleigh%20Scattering Rayleigh%20Scattering)
  (bind _skyatmosphere (Variables|Default|GetSkyAtmosphere)
    (:then
      (Class|SkyAtmosphereComponent|SetRayleighScattering (Variables|/Script/Engine.SkyAtmosphere|GetSkyAtmosphereComponent _skyatmosphere) Rayleigh%20Scattering))
    (:else
      (Development|PrintString "Assign SkyAtmosphere value")))
  (bind _postprocessvolume (Variables|Default|GetPostProcessVolume)
    (:then
      (Utilities|Struct|SetmembersinPostProcessSettings (Variables|/Script/Engine.PostProcessVolume|GetSettings _postprocessvolume) Exposure%20Compensation))
    (:else
      (Development|PrintString "Assign PostProcess value")))
  (bind _volumeticclouds (Variables|Default|GetVolumeticClouds)
    (:then
      (Variables|Default|GetCloudMat
        (:then
          _)
        (:else
          (bind _returnvalue (Rendering|Material|CreateDynamicMaterialInstance "/Game/BP/Weather/Assets/m_SimpleVolumetricCloud_Inst.m_SimpleVolumetricCloud_Inst" "MClouds" "None" :!class /Script/Engine.KismetMaterialLibrary))
          (bind _output_get (Variables|Default|SetCloudMat _returnvalue))))
      (Rendering|Material|SetMaterial (Variables|/Script/Engine.VolumetricCloud|GetVolumetricCloudComponent _volumeticclouds) _output_get)
      (Rendering|Material|SetScalarParameterValue _output_get "Cloud_GlobalCoverage" CloudDensityOffset :!class /Script/Engine.MaterialInstanceDynamic))
    (:else
      (Development|PrintString "Assign VolumeticClouds value"))))

(fn ColorInterptoConstant
  (params (InColor :type Linear%20Color%20Structure) (InColor2 :type Linear%20Color%20Structure) (InputPin :type Float%20%28double-precision%29))
  (bind (_r _g _b _a) (Math|Color|BreakColor InColor))
  (bind (_r_2 _g_2 _b_2 _a_2) (Math|Color|BreakColor InColor2))
  (bind _returnvalue (Utilities|Time|GetWorldDeltaSeconds))
  (return (Utilities|Struct|MakeLinearColor (Math|Interpolation|FInterptoConstant _r _r_2 _returnvalue InputPin) (Math|Interpolation|FInterptoConstant _g _g_2 _returnvalue InputPin) (Math|Interpolation|FInterptoConstant _b _b_2 _returnvalue InputPin) (Math|Interpolation|FInterptoConstant _a _a_2 _returnvalue InputPin))))