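; Rain and thunderstorm actor that keeps Niagara rain above the player, with ToggleRain switching rain and its sound.
; Enabling rain finds a PostProcessVolume and starts an endless randomly timed thunder loop, which disabling does not stop.
; Each strike moves a lightning plane randomly ahead of the camera, picks one of two textures, plays sound and a timeline-driven material fade.
; The loop then briefly overrides the volume's exposure compensation for a flash.
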(event Custom|Strike
  (|ReLocate
    (:OutputPin
      (|Change_Texture
        (:OutputPin
          (Audio|PlaySound2D (Variables|Default|GetThunderSound) 1.0 1.0 0.0 0 0)
          (bind _y (Timeline|Thunder_strike PlayFromStart)
            (:Update
              (Rendering|Material|SetScalarParameterValueonMaterials (Variables|Default|GetThunder_plane) "y" _y))))))))

(event Custom|ToggleRain
  (params (Enable/Disable :type Boolean))
  (bind _ns_rain (Variables|Default|GetNS_Rain))
  (if Enable/Disable
    (Variables|Default|SetRainEnabled true)
    (Components|Activation|Activate _ns_rain false)
    (Transformation|DetachFromComponent (Variables|Default|GetNS_Rain) "KeepRelative" "KeepWorld" "KeepWorld" true)
    (Variables|Default|GetPP_Volume
      (:then
        (|Thunder :!label _label))
      (:else
        (|GetPostProcess
          (:OutputPin
            (goto _label))
          (:NotPostProcess
            (Development|PrintString "No PP Set")))))
    (else
      (Variables|Default|SetRainEnabled false)
      (Components|Activation|Deactivate _ns_rain))))

(event EventBeginPlay)

(event Collision|EventActorBeginOverlap
  (params (OtherActor :type Actor%20Object%20Reference)))

(event EventTick
  (params (DeltaSeconds :type Float%20%28single-precision%29))
  (Transformation|SetWorldLocation (Variables|Default|GetNS_Rain) (+ (Transformation|GetActorLocation (Game|GetPlayerCharacter 0)) "0.000000,0.000000,1000.000000") false false))

(fn ConstructionScript)