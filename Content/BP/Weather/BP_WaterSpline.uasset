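; BP_WaterSpline is a weather actor that runs a water drop Niagara effect along a spline path.
; On BeginPlay it passes DropRate to the effect's user parameter.
; Each Tick it moves the effect to the current spline distance, then advances that distance by NSMoveSpeed plus random jitter, without delta-time scaling.
; Past the spline's end, the distance wraps to a small random offset near the start.
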(event EventBeginPlay
  (Niagara|SetNiagaraVariable(Float) (Variables|Default|GetNS_WaterSpline) "User.DropRate" (Variables|Default|GetDropRate)))

(event Collision|EventActorBeginOverlap
  (params (OtherActor :type Actor%20Object%20Reference)))

(event EventTick
  (params (DeltaSeconds :type Float%20%28single-precision%29))
  (bind _returnvalue (Math|Random|RandomFloatinRange 0.0 2e+01))
  (Transformation|SetWorldLocation (Variables|Default|GetNS_WaterSpline) (Spline|GetLocationatDistanceAlongSpline (Variables|Default|GetSpline) (Variables|Default|GetDistance) "World") false false)
  (bind _output_get (Variables|Default|SetDistance (+ (Variables|Default|GetDistance) (Variables|Default|GetNS_MoveSpeed) _returnvalue)))
  (if (> _output_get (Spline|GetSplineLength (Variables|Default|GetSpline)))
    (Variables|Default|SetDistance _returnvalue)))

(fn ConstructionScript)