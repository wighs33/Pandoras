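; Chapter 0 trigger that plays the player character's stand-up animation as a scripted moment without player control.
; The first overlap on its collision component, after a short delay, disables input, plays the montage, then re-enables input after a fixed delay timed in place of a completion callback.
; The IsPlayerMessage check on the overlapping actor has empty branches, and the dialogue widget logic is disconnected, so no dialogue appears.
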(event OnComponentBeginOverlap(CollisionComponent)
  (params (OverlappedComponent :type Primitive%20Component%20Object%20Reference) (OtherActor :type Actor%20Object%20Reference) (OtherComp :type Primitive%20Component%20Object%20Reference) (OtherBodyIndex :type Integer) (bFromSweep :type Boolean) (SweepResult :type Hit%20Result%20Structure%20%28by%20ref%29))
  (Utilities|FlowControl|Delay 1.0)
  (Utilities|FlowControl|DoOnce false
    (:Completed
      ;[0.15 0.15 0.15 0.5] 플레이어 캐릭터의 일어나는 애니메이션 (조종불가)
      (Input|DisableInput (Game|GetPlayerCharacter 0) (Game|GetPlayerController 0))
      (bind _returnvalue (Class|CharacterInterface|IsPlayer(Message) OtherActor))
      (if _returnvalue
        _
        (else
          _))
      (Animation|PlayAnimMontage (Game|GetPlayerCharacter 0) "/Game/Characters/Mannequins/Animations/Mixamo/StandUp_UE_Montage.StandUp_UE_Montage" 1.0 "None")
      (Utilities|FlowControl|Delay 8.2)
      ;[0.15 0.15 0.15 0.5] 대화창 끝나고 조종 가능
      (Input|EnableInput (Game|GetPlayerCharacter 0) (Game|GetPlayerController 0)))))

(event EventBeginPlay)

(event Collision|EventActorBeginOverlap
  (params (OtherActor :type Actor%20Object%20Reference)))

(event EventTick
  (params (DeltaSeconds :type Float%20%28single-precision%29)))

(fn ConstructionScript)