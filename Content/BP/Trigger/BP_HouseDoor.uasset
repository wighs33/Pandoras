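; BP_HouseDoor is a house door trigger actor that shows an interaction widget when a player comes near.
; When the InteractCollider begins overlapping an actor that passes the IsPlayerMessage check for the local character, it shows the Widget and hides the MaterialBillboard.
; Any end overlap reverses this without a player check, hiding the widget and showing the billboard again.
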(event OnComponentBeginOverlap(InteractCollider)
  (params (OverlappedComponent :type Primitive%20Component%20Object%20Reference) (OtherActor :type Actor%20Object%20Reference) (OtherComp :type Primitive%20Component%20Object%20Reference) (OtherBodyIndex :type Integer) (bFromSweep :type Boolean) (SweepResult :type Hit%20Result%20Structure%20%28by%20ref%29))
  ;[0.15 0.15 0.15 0.5] 로컬 캐릭터인 지 체크
  (bind _returnvalue (Class|CharacterInterface|IsPlayer(Message) OtherActor))
  (if _returnvalue
    ;[0.15 0.15 0.15 0.5] 위젯은 표시, 빌보드는 숨기기
    (Development|SetHiddeninGame (Variables|Default|GetWidget) false false)
    (Development|SetHiddeninGame (Variables|Default|GetMaterialBillboard) true false)))

(event OnComponentEndOverlap(InteractCollider)
  (params (OverlappedComponent :type Primitive%20Component%20Object%20Reference) (OtherActor :type Actor%20Object%20Reference) (OtherComp :type Primitive%20Component%20Object%20Reference) (OtherBodyIndex :type Integer))
  ;[0.15 0.15 0.15 0.5] 위젯은 숨기기, 빌보드는 표시
  (Development|SetHiddeninGame (Variables|Default|GetWidget) true false)
  (Development|SetHiddeninGame (Variables|Default|GetMaterialBillboard) false false))

(event EventBeginPlay)

(event Collision|EventActorBeginOverlap
  (params (OtherActor :type Actor%20Object%20Reference)))

(event EventTick
  (params (DeltaSeconds :type Float%20%28single-precision%29)))

(fn ConstructionScript)