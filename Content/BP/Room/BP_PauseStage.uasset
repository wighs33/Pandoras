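; BP_PauseStage is the pause-room actor where the player's character is previewed behind the inventory and skill-tree screens.
; Opening either, if alive, stops movement, waits out root motion, moves only the character mesh onto the stage, and switches view and HUD.
; The camera eases between spring arms for body-part focus, and click-dragging rotates the mesh, which eases back after a retriggerable delay.
; Exiting restores the mesh transform, input, view and in-game HUD.
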(event Input|EnhancedActionEvents|EnhancedInputActionIA_Inventory
  (params (ActionValue :type Boolean) (ElapsedSeconds :type Float%20%28double-precision%29) (TriggeredSeconds :type Float%20%28double-precision%29) (InputAction :type Input%20Action%20Object%20Reference :default "/Game/ThirdPerson/Input/Actions/IA_Inventory.IA_Inventory"))
  (:Started
    (Utilities|TogglePauseMode)
    ;[0.15 0.15 0.15 0.5] 인벤토리 화면UI로 전환
    (Class|HudInterface|SwitchtoInventoryUI(Message) (HUD|GetHUD (Game|GetPlayerController 0)) self)))

(event Input|EnhancedActionEvents|EnhancedInputActionIA_SkillTree
  (params (ActionValue :type Boolean) (ElapsedSeconds :type Float%20%28double-precision%29) (TriggeredSeconds :type Float%20%28double-precision%29) (InputAction :type Input%20Action%20Object%20Reference :default "/Game/ThirdPerson/Input/Actions/IA_SkillTree.IA_SkillTree"))
  (:Started
    (Utilities|TogglePauseMode)
    ;[0.15 0.15 0.15 0.5] 스킬 메뉴 화면UI로 전환
    (Class|HudInterface|SwitchtoSkillMenu(Message) (HUD|GetHUD (Game|GetPlayerController 0)))))

(event Input|EnhancedActionEvents|EnhancedInputActionIA_Look
  (params (ActionValue :type Vector%202D%20Structure) (ElapsedSeconds :type Float%20%28double-precision%29) (TriggeredSeconds :type Float%20%28double-precision%29) (InputAction :type Input%20Action%20Object%20Reference :default "/Game/ThirdPerson/Input/Actions/IA_Look.IA_Look"))
  ;[0.15 0.15 0.15 0.5] 메시 회전 중 플래그 ON일 때 메시를 프레임에 비례하여 회전
  (if (Variables|Default|GetbMeshRotating)
    (Transformation|AddRelativeRotation (Variables|/Script/Engine.Character|GetMesh (Variables|Default|GetPlayerCharacter)) (Math|Rotator|MakeRotator 0.0 0.0 (* (.x ActionValue) (Utilities|Time|GetWorldDeltaSeconds) -1e+02)) false false)
    (Utilities|FlowControl|RetriggerableDelay 5.0)
    ;[0.15 0.15 0.15 0.5] 메시 회전 리셋
    (Class|InventoryRoom|ResetMeshRotation)))

(event EventBeginPlay
  ;[0.15 0.15 0.15 0.5] 미리 캐릭터 입력 활성화 (인벤토리 키 입력 받기 위함)
  (Input|EnableInput (Game|GetPlayerController 0)))

(event Collision|EventActorBeginOverlap
  (params (OtherActor :type Actor%20Object%20Reference)))

(event EventEnterPauseMode
  (bind _returnvalue (Game|GetPlayerController 0))
  (bind _playerposition (Variables|Default|GetPlayerPosition))
  (bind _returnvalue_2 (Transformation|GetWorldTransform _playerposition))
  ;[0.15 0.15 0.15 0.5] 플레이어의 캐릭터 저장
  (bind _output_get (Variables|Default|SetPlayerCharacter (Game|GetPlayerCharacter 0)))
  ;[0.15 0.15 0.15 0.5] 캐릭터 입력 비활성화 후 3D클릭 활성화
  (Input|DisableInput _output_get _returnvalue)
  (Variables|/Script/Engine.PlayerController|SetbEnableClickEvents _returnvalue true)
  (AI|Navigation|StopMovement) ; 캐릭터의 움직임 완전히 멈추기
  (Variables|Default|SetbInPauseMode true)
  ;[0.15 0.15 0.15 0.5] 인게임에서 메시와 캐릭터의 상대적인 위치 저장
  (Variables|Default|SetMeshRelativeTransformOrigin (Transformation|GetRelativeTransform (Variables|/Script/Engine.Character|GetMesh (Variables|Default|GetPlayerCharacter))))
  ;[0.15 0.15 0.15 0.5] 메시만 인벤토리로 옮긴 후에 캐릭터와 메시의 상대적인 위치 저장
  (Transformation|SetWorldLocationAndRotation (Variables|/Script/Engine.Character|GetMesh (Variables|Default|GetPlayerCharacter)) (.location _returnvalue_2) (.rotation _returnvalue_2) false false)
  (Variables|Default|SetMeshRelativeTransformInventory (Transformation|GetRelativeTransform (Variables|/Script/Engine.Character|GetMesh (Variables|Default|GetPlayerCharacter))))
  ;[0.15 0.15 0.15 0.5] 인벤토리 내부 카메라의 시점으로 전환
  (Game|Player|SetViewTargetwithBlend (Game|GetPlayerController 0) self 0.0 "VTBlend_Linear" 0.0 false)
  ;[0.15 0.15 0.15 0.5] UI입력 활성화
  (Class|HudInterface|ToggleUIInput(Message) (HUD|GetHUD (Game|GetPlayerController 0)) true))

(event EventExitPauseMode
  (bind _returnvalue (Game|GetPlayerController 0))
  (bind _returnvalue_2 (Game|GetPlayerController 0))
  (bind _meshrelativetransformorigin (Variables|Default|GetMeshRelativeTransformOrigin))
  (bind _playercharacter (Variables|Default|GetPlayerCharacter))
  (bind _returnvalue_3 (HUD|GetHUD _returnvalue_2))
  ;[0.15 0.15 0.15 0.5] 메시의 회전을 멈추고 캐릭터의 메시를 인게임에서의 위치로 다시 이동
  (bind _playercharacter_2 (Variables|Default|GetPlayerCharacter)
    (:then
      (Class|InventoryRoom|StopMeshRotation)
      (Transformation|SetRelativeLocationAndRotation (Variables|/Script/Engine.Character|GetMesh _playercharacter_2) (.location _meshrelativetransformorigin) (.rotation _meshrelativetransformorigin) false false)
      ;[0.15 0.15 0.15 0.5] 캐릭터 입력 다시 활성화하고 캐릭터의 시점으로 다시 전환
      (Input|EnableInput _playercharacter _returnvalue)
      (Game|Player|SetViewTargetwithBlend _returnvalue _playercharacter 0.0 "VTBlend_Linear" 0.0 false)
      (Variables|Default|SetbInPauseMode false)
      ;[0.15 0.15 0.15 0.5] 캐릭터의 움직임을 걷기로 설정
      (Pawn|Components|CharacterMovement|SetMovementMode (Variables|/Script/Engine.Character|GetCharacterMovement (Variables|Default|GetPlayerCharacter)) "MOVE_Walking" 0)
      ;[0.15 0.15 0.15 0.5] 인게임 HUD로 전환하며 UI입력과 3D클릭 비활성화
      (Class|HudInterface|SwitchtoinGameHud(Message) _returnvalue_3)
      (Class|HudInterface|ToggleUIInput(Message) _returnvalue_3 false)
      (Variables|/Script/Engine.PlayerController|SetbEnableClickEvents (Game|GetPlayerController 0) false))
    (:else)))

(event EventTick
  (params (DeltaSeconds :type Float%20%28single-precision%29)))

(event EventChangeFocusPoint
  (params (focus_point :type ECharacterFocusPoint%20Enum :default "Main"))
  ;[0.15 0.15 0.15 0.5] 메시 회전 리셋
  (Class|InventoryRoom|ResetMeshRotation)
  ;[0.15 0.15 0.15 0.5] [포커싱 시점 키워드]에 따라 다른 스프링암에 카메라 부착
  (Transformation|AttachComponentToComponent (Variables|Default|GetCamera) (Utilities|Select :Index focus_point :Main (Variables|Default|GetMainSpringArm) :Weapon (Variables|Default|GetWeaponSpringArm) :Head (Variables|Default|GetHeadSpringArm) :Hands (Variables|Default|GetHandSpringArm) :Feet (Variables|Default|GetFootSpringArm)) "None" "KeepWorld" "KeepWorld" "KeepWorld" true)
  ;[0.15 0.15 0.15 0.5] 카메라를 부착된 지점의 원점으로 서서히 이동
  (Components|MoveComponentTo (Variables|Default|GetCamera) "0, 0, 0" "0, 0, 0" true false 0.4 false))

(event EventOnCapsuleClicked
  (params (ClickedComp :type Primitive%20Component%20Object%20Reference) (ButtonPressed :type Key%20Structure :default "None"))
  (Variables|Default|SetbMeshRotating true))

(event EventOnCapsuleReleased
  (params (ClickedComp :type Primitive%20Component%20Object%20Reference) (ButtonPressed :type Key%20Structure :default "None"))
  (Variables|Default|SetbMeshRotating false))

(event EventResetMeshRotation
  (bind _meshrelativetransforminventory (Variables|Default|GetMeshRelativeTransformInventory))
  ;[0.15 0.15 0.15 0.5] 인벤토리 열림 여부 체크
  (if (Variables|Default|GetbInPauseMode)
    ;[0.15 0.15 0.15 0.5] 메시를 인벤토리 스폰시점의 위치로 복귀 or stop
    (Components|MoveComponentTo (Variables|/Script/Engine.Character|GetMesh (Variables|Default|GetPlayerCharacter)) (.location _meshrelativetransforminventory) (.rotation _meshrelativetransforminventory) true true 0.8 true)))

(event EventStopMeshRotation
  (bind _meshrelativetransforminventory (Variables|Default|GetMeshRelativeTransformInventory))
  ;[0.15 0.15 0.15 0.5] 메시를 인벤토리 스폰시점의 위치로 복귀 or stop
  (Components|MoveComponentTo (Variables|/Script/Engine.Character|GetMesh (Variables|Default|GetPlayerCharacter)) (.location _meshrelativetransforminventory) (.rotation _meshrelativetransforminventory) true true 0.8 true) ; enters at Stop
)

(event Input|KeyboardEvents|1
  (params (Key :type Key%20Structure :default "None"))
  (:Pressed
    (Class|InventoryRoom|ChangeFocusPoint "Main")))

(event Input|KeyboardEvents|2
  (params (Key :type Key%20Structure :default "None"))
  (:Pressed
    (Class|InventoryRoom|ChangeFocusPoint "Weapon")))

(fn ConstructionScript)