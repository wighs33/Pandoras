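; Save point actor that saves the player's character data on interaction.
; Overlapping the interact collider as the player swaps the billboard for a "Save" prompt widget and enables input; any overlap end reverses this without a cast check.
; While enabled, IA_AreaOfEffect calls SaveCharacterData on player 0's character, shows a completion notification and swaps the SkyT021 material to NEON2, with no revert.
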(event OnComponentBeginOverlap(InteractCollider)
  (params (OverlappedComponent :type Primitive%20Component%20Object%20Reference) (OtherActor :type Actor%20Object%20Reference) (OtherComp :type Primitive%20Component%20Object%20Reference) (OtherBodyIndex :type Integer) (bFromSweep :type Boolean) (SweepResult :type Hit%20Result%20Structure%20%28by%20ref%29))
  ;[0.15 0.15 0.15 0.5] 로컬 캐릭터인 지 체크
  (Utilities|Casting|CastToBP_PandorasCharacter_Player OtherActor)
  ;[0.15 0.15 0.15 0.5] 위젯은 표시, 빌보드는 숨기기
  (Development|SetHiddeninGame (Variables|Default|GetWidget) false false)
  (Development|SetHiddeninGame (Variables|Default|GetMaterialBillboard) true false)
  (Input|EnableInput (Game|GetPlayerController 0)))

(event OnComponentEndOverlap(InteractCollider)
  (params (OverlappedComponent :type Primitive%20Component%20Object%20Reference) (OtherActor :type Actor%20Object%20Reference) (OtherComp :type Primitive%20Component%20Object%20Reference) (OtherBodyIndex :type Integer))
  ;[0.15 0.15 0.15 0.5] 위젯은 숨기기, 빌보드는 표시
  (Development|SetHiddeninGame (Variables|Default|GetWidget) true false)
  (Development|SetHiddeninGame (Variables|Default|GetMaterialBillboard) false false)
  (Input|DisableInput (Game|GetPlayerController 0)))

(event Custom|ChangeLightColor
  (Rendering|Material|SetMaterial (Variables|Default|Getsky_t_021) 0 "/Game/Fab/SKY_T_021/NEON2.NEON2"))

(event Input|EnhancedActionEvents|EnhancedInputActionIA_AreaOfEffect
  (params (ActionValue :type Vector%202D%20Structure) (ElapsedSeconds :type Float%20%28double-precision%29) (TriggeredSeconds :type Float%20%28double-precision%29) (InputAction :type Input%20Action%20Object%20Reference :default "/Game/ThirdPerson/Input/Actions/IA_AreaOfEffect.IA_AreaOfEffect"))
  (:Started
    (bind _asbp_pandoras_character_player (Utilities|Casting|CastToBP_PandorasCharacter_Player (Game|GetPlayerCharacter 0)))
    (Class|PandorasCharacterBase|SaveCharacterData _asbp_pandoras_character_player)
    (Class|CharacterInterface|ShowCharacterNotification(Message) _asbp_pandoras_character_player (Utilities|Struct|MakeNotification "Save Complete!" "/Game/BP/UI/Asset/saveicon.saveicon"))
    (CallFunction|ChangeLightColor)))

(event EventBeginPlay
  (bind _aswdg_interact_tip (Utilities|Casting|CastToWDG_InteractTip (UserInterface|GetWidget (Variables|Default|GetWidget))))
  (Default|ChangeText _aswdg_interact_tip "Save"))

(event Collision|EventActorBeginOverlap
  (params (OtherActor :type Actor%20Object%20Reference)))

(event EventTick
  (params (DeltaSeconds :type Float%20%28single-precision%29)))

(fn ConstructionScript)