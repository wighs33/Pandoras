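; Tower-top item box that players open once to collect item abilities, a house key and a parachute.
; Overlap enables interact input, sets ownership and shows the local prompt widget.
; Interaction reaches a multicast through the server, which plays effects and opens the lid, while authority alone grants items and minor experience.
; The multicast also shows notifications and a descent tip, setting key and parachute flags on each machine's player 0 character.
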(event Input|EnhancedActionEvents|EnhancedInputActionIA_Interact
  (params (ActionValue :type Boolean) (ElapsedSeconds :type Float%20%28double-precision%29) (TriggeredSeconds :type Float%20%28double-precision%29) (InputAction :type Input%20Action%20Object%20Reference :default "/Game/ThirdPerson/Input/Actions/IA_Interact.IA_Interact"))
  (bind _interactingactor (Variables|Default|GetInteractingActor))
  (:Started
    ;[0.15 0.15 0.15 0.5] 서버와 클라 분기
    (Networking|SwitchHasAuthority
      (:Authority
        ;[0.15 0.15 0.15 0.5] 수집 동기화
        (Class|ItemBox|CollectMulticast _interactingactor))
      (:Remote
        (Class|ItemBox|CollectServer _interactingactor)))))

(event EventBeginPlay)

(event Collision|EventActorBeginOverlap
  (params (OtherActor :type Actor%20Object%20Reference)))

(event EventTick
  (params (DeltaSeconds :type Float%20%28single-precision%29)))

(event EventOnColliderBeginOverlap
  (params (OverlappedComp :type Primitive%20Component%20Object%20Reference) (OtherActor :type Actor%20Object%20Reference) (OtherComp :type Primitive%20Component%20Object%20Reference) (OtherBodyIndex :type Integer) (bFromSweep :type Boolean) (SweepResult :type Hit%20Result%20Structure%20%28by%20ref%29))
  ;[0.15 0.15 0.15 0.5] 플레이어인 지 체크
  (bind _returnvalue (Class|CharacterInterface|IsPlayer(Message) OtherActor))
  (if _returnvalue
    ;[0.15 0.15 0.15 0.5] 해당 플레이어 저장
    (Variables|Default|SetInteractingActor OtherActor)
    ;[0.15 0.15 0.15 0.5] 입력 활성화
    (Input|EnableInput (Game|GetPlayerController 0))
    ;[0.15 0.15 0.15 0.5] 해당 액터와 함께 리플리케이션 되도록 바인딩
    (Actor|SetOwner (Variables|Default|GetInteractingActor))
    ;[0.15 0.15 0.15 0.5] 로컬 캐릭터인 지 체크
    (bind _returnvalue_2 (Class|CharacterInterface|IsLocalCharacter(Message) (Variables|Default|GetInteractingActor)))
    (if _returnvalue_2
      ;[0.15 0.15 0.15 0.5] 위젯은 표시, 빌보드는 숨기기
      (Development|SetHiddeninGame (Variables|Default|GetWidget) false false)
      (Development|SetHiddeninGame (Variables|Default|GetMaterialBillboard) true false))))

(event EventOnColliderEndOverlap
  (params (OverlappedComp :type Primitive%20Component%20Object%20Reference) (OtherActor :type Actor%20Object%20Reference) (OtherComp :type Primitive%20Component%20Object%20Reference) (OtherBodyIndex :type Integer))
  (Variables|Default|SetInteractingActor 0)
  (Input|DisableInput 0)
  ;[0.15 0.15 0.15 0.5] 위젯은 숨기기, 빌보드는 표시
  (Development|SetHiddeninGame (Variables|Default|GetWidget) true false)
  (Development|SetHiddeninGame (Variables|Default|GetMaterialBillboard) false false))

(event EventCollectServer
  (params (OwnerActor :type Actor%20Object%20Reference))
  (Class|ItemBox|CollectMulticast OwnerActor))

(event EventCollectMulticast
  (params (OwnerActor :type Actor%20Object%20Reference))
  (bind _returnvalue (Ability|GetAbilitySystemComponent OwnerActor))
  ;[0.15 0.15 0.15 0.5] 하나의 상자는 한번만 획득
  (Utilities|FlowControl|DoOnce false
    (:Completed
      ;[0.15 0.15 0.15 0.5] 이펙트와 사운드
      (|FxandSound
        (:OutputPin
          ;[0.15 0.15 0.15 0.5] 뚜껑 열기
          (Components|MoveComponentTo (Variables|Default|GetLid) "-60.000000,-60.000000,0.000000" "0, 0, 0" true true 0.4 false)
          ;[0.15 0.15 0.15 0.5] 서버와 클라 분기
          (Networking|SwitchHasAuthority
            (:Authority
              ;[0.15 0.15 0.15 0.5] 장착 어빌리티 클래스 각각
              (for _array_element (Variables|Default|GetItemAbilityClasses)
                ;[0.15 0.15 0.15 0.5] ASC 유효성 체크
                (Utilities|IsValid _returnvalue
                  (:Is%20Valid
                    ;[0.15 0.15 0.15 0.5] 아이템 데이터를 플레이어에  저장
                    (Class|ItemWielderInterface|AddItemtoPlayerState(Message) OwnerActor _array_element)
                    ;[0.15 0.15 0.15 0.5] HUD 아이템 획득 알람 표시
                    (|ShowNotification OwnerActor _array_element))))
              ;[0.15 0.15 0.15 0.5] 오픈한 사람에게 소량 경험치 GE 적용
              (GameplayEffects|ApplyGameplayEffectToSelf :self _returnvalue :GameplayEffectClass "/Game/BP/Ability/GE_MinorExperience.GE_MinorExperience_C"))
            (:Remote
              _))
          ;[0.15 0.15 0.15 0.5] 빌보드 시각화 끄기
          (Rendering|SetVisibility (Variables|Default|GetMaterialBillboard) false true)
          ;[0.15 0.15 0.15 0.5] 충돌 트리거 끄기
          (Collision|SetCollisionEnabled (Variables|Default|GetPlayerCollider) "NoCollision")
          ;[0.15 0.15 0.15 0.5] 열쇠와 낙하산 얻기
          (Class|CharacterInterface|ShowCharacterNotification(Message) OwnerActor (Utilities|Struct|MakeNotification "House Key Collected" "/Game/BP/UI/Asset/housekey.housekey"))
          (Class|CharacterInterface|ShowCharacterNotification(Message) OwnerActor (Utilities|Struct|MakeNotification "Parachute Collected" "/Game/BP/UI/Asset/parachute.parachute"))
          (Class|HudInterface|ShowTip(Message) (HUD|GetHUD (Game|GetPlayerController 0)) "<Input>낙하산(V키)</>으로 낙하한 후 <Input>오두막집</>으로 이동하자" 8.0)
          (bind _asbp_pandoras_character (Utilities|Casting|CastToBP_PandorasCharacter (Game|GetPlayerCharacter 0)))
          (Variables|/Game/ThirdPerson/Blueprints/BP_PandorasCharacter.BP_PandorasCharacter_C|SetHasHouseKey _asbp_pandoras_character true)
          (Variables|/Game/ThirdPerson/Blueprints/BP_PandorasCharacter.BP_PandorasCharacter_C|SetHasParachute _asbp_pandoras_character true))))))

(fn ConstructionScript)